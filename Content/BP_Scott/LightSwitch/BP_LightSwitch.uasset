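; BP_LightSwitch is an interactable light switch that turns a spotlight on and off.
; Each Interaction event alternates through a FlipFlop, playing a sound at the switch and showing or hiding the SpotLight.
; The LightSwitch_TL timeline plays or reverses alongside it, interpolating the LightSwitch component's pitch to animate the flick.
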(event `/Game/FirstPerson/Blueprints/BPI_Interact.Interaction`
  (bind _spotlight (`self.SpotLight`))
  (`/Engine/EditorBlueprintResources/StandardMacros.FlipFlop`
    (:`A`
      (`GameplayStatics.PlaySoundAtLocation` null (`SceneComponent.K2_GetComponentLocation` (`self.LightSwitch`)) (struct) 1.0 1.0 0.0 null null null null)
      (`SceneComponent.SetVisibility` _spotlight true false)
      (bind (_direction _lightswitchalpha) (`Timeline|LightSwitch_TL` :!label _label)
        (:`Update`
          (`SceneComponent.K2_SetRelativeRotation` (`self.LightSwitch`) (`KismetMathLibrary.MakeRotator` 0.0 (`KismetMathLibrary.Lerp` 10.0 -10.0 _lightswitchalpha)) false false))))
    (:`B`
      (`GameplayStatics.PlaySoundAtLocation` null (`SceneComponent.K2_GetComponentLocation` (`self.LightSwitch`)) (struct) 1.0 1.0 0.0 null null null null)
      (`SceneComponent.SetVisibility` _spotlight false false)
      (goto _label :!via `Reverse`))))

(fn `UserConstructionScript`)