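; BP_Bed is an interactable bed that moves the first-person player to a set spot when used.
; BeginPlay caches the player character, and the Interaction event teleports it to TpPos.
; The TpPos location is converted from the bed's local space to world space, while its rotation is applied untransformed.
; The box overlap event is empty, and IsPlayer? is a stub returning false.
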(event `self.ReceiveBeginPlay`
  (bind _asbp_first_person_character (cast `/Game/FirstPerson/Blueprints/BP_FirstPersonCharacter` (`GameplayStatics.GetPlayerCharacter` 0)))
  (set `self.Char Ref` _asbp_first_person_character))

(event `self.Box.OnComponentBeginOverlap`
  (params (OverlappedComponent :type "PrimitiveComponent Object Reference") (OtherActor :type "Actor Object Reference") (OtherComp :type "PrimitiveComponent Object Reference") (OtherBodyIndex :type Integer) (bFromSweep :type Boolean) (SweepResult :type "HitResult Structure (by ref)")))

(event `/Game/FirstPerson/Blueprints/BPI_Interact.Interaction`
  (bind (_tp_pos_location _tp_pos_rotation) (`KismetMathLibrary.BreakTransform` (`self.tp pos`)))
  (bind _asbp_first_person_character (cast `/Game/FirstPerson/Blueprints/BP_FirstPersonCharacter` (`self.Char Ref`)))
  (`self.K2_SetActorLocationAndRotation` _asbp_first_person_character (`KismetMathLibrary.TransformLocation` (`self.GetTransform`) _tp_pos_location) _tp_pos_rotation false false))

(fn `IsPlayer?`
  (returns (`Yes/No` :type Boolean))
  (return false))

(fn `UserConstructionScript`)