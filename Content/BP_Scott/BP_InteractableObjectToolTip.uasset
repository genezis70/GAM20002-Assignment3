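; Interactable-object actor that shows an on-screen tooltip while the player stands inside its Box trigger.
; Box overlap begin checks the other actor through the IsPlayer message, lazily creates a cached WDG_ToolTip widget and adds it to the viewport.
; Overlap end runs the same check and removes the widget from the viewport, keeping the instance for reuse.
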(event `self.Box.OnComponentBeginOverlap`
  (params (OverlappedComponent :type "PrimitiveComponent Object Reference") (OtherActor :type "Actor Object Reference") (OtherComp :type "PrimitiveComponent Object Reference") (OtherBodyIndex :type Integer) (bFromSweep :type Boolean) (SweepResult :type "HitResult Structure (by ref)"))
  (bind _yes_no (message `/Game/BP_Scott/BPI_Player.IsPlayer?` OtherActor))
  (if _yes_no
    (`self.WDG_ToolTipWidget`
      (:`then`
        _)
      (:`else`
        (bind _returnvalue (`|CreateWidget` "/Game/BP_Scott/WDG_ToolTip.WDG_ToolTip_C"))
        (set `self.WDG_ToolTipWidget` _returnvalue)))
    (`UserWidget.AddToViewport` (`self.WDG_ToolTipWidget`) 0)))

(event `self.Box.OnComponentEndOverlap`
  (params (OverlappedComponent :type "PrimitiveComponent Object Reference") (OtherActor :type "Actor Object Reference") (OtherComp :type "PrimitiveComponent Object Reference") (OtherBodyIndex :type Integer))
  (bind _yes_no (message `/Game/BP_Scott/BPI_Player.IsPlayer?` OtherActor))
  (if _yes_no
    (bind _wdg_tooltipwidget (`self.WDG_ToolTipWidget`)
      (:`then`
        (if (`Widget.IsInViewport` _wdg_tooltipwidget)
          (`Widget.RemoveFromParent` (`self.WDG_ToolTipWidget`))))
      (:`else`))))

(fn `UserConstructionScript`)