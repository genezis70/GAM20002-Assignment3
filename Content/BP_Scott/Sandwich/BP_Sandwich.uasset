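; BP_Sandwich is an interactable actor that reveals a sandwich once no remaining items are left.
; The Sandwich component starts hidden at BeginPlay.
; On Interaction it reads Remaining from BP_FirstPersonGameMode and shows the sandwich if the count is zero.
; Otherwise it creates a WB_RemainingItems widget and removes it after a three-second delay.
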(event `self.ReceiveBeginPlay`
  (`SceneComponent.SetVisibility` (`self.Sandwich`) false false))

(event `/Game/FirstPerson/Blueprints/BPI_Interact.Interaction`
  (bind _asbp_first_person_game_mode (cast `/Game/FirstPerson/Blueprints/BP_FirstPersonGameMode` (`GameplayStatics.GetGameMode`)))
  (if (== (`/Game/FirstPerson/Blueprints/BP_FirstPersonGameMode.Remaining` _asbp_first_person_game_mode) 0)
    (`SceneComponent.SetVisibility` (`self.Sandwich`) true false)
    (else
      (bind _returnvalue (`|CreateWidget` "/Game/BP_Scott/Sandwich/WB_RemainingItems.WB_RemainingItems_C"))
      (`UserWidget.AddToViewport` _returnvalue 0)
      (`KismetSystemLibrary.Delay` 3.0)
      (`Widget.RemoveFromParent` _returnvalue))))

(fn `UserConstructionScript`)